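; HoloLens player pawn for a world-builder app, running the AR session, UXT hand interactions, spawner UI and toolbox.
; Tick traces head and eye gaze, detects blinks, and poses hand meshes from keypoints, mirroring the left, while the spawner enables them.
; Hold and voice inputs message BPi_HoloLens actors via hand-cursor overlaps or gaze hits.
; It also manages local-store anchor pins and toggles spatial-mesh wireframe.
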(event `self.ReceiveBeginPlay`
  (`self.PrepareForAR`))

(event `self.ReceiveTick`
  (params (DeltaSeconds :type "Float (single-precision)"))
  (bind _righthand (`self.RightHand`))
  (bind _righthand_2 (`self.RightHand`))
  ;[1 1 1] We will track the eyes and head every frame
  (`self.HeadOrientationTracking`)
  (`self.EyeGazeTracking`)
  (if (`self.RenderHands`)
    ;[1 1 1] Track hands every frame
    (`self.TrackHands`)
    ;[1 1 1] If rendering hands, make sure they are visible. If not, hide them.
    (if (not (`SceneComponent.IsVisible` _righthand_2))
      (`SceneComponent.SetVisibility` _righthand_2 true true)
      (`SceneComponent.SetVisibility` (`self.LeftHand`) true true))
    (elif (`SceneComponent.IsVisible` _righthand)
      (`SceneComponent.SetVisibility` _righthand false true)
      (`SceneComponent.SetVisibility` (`self.LeftHand`) false true))))

(event `PrepareForAR`
  ;[1 1 1] Starting and stopping the AR Session
  (`ARBlueprintLibrary.StartARSession` "/Game/WorldBuilder/Assets/AR_SessionConfig.AR_SessionConfig")
  ;[1 1 1] Spawn and configure Hand interactions
  (`self.SpawnHandInteractions`)
  (`self.ConfigureGestures`)
  ;[1 1 1] Spawn the UI to the map
  (`self.SpawnUI`))

(event `self.ReceiveEndPlay`
  (params (EndPlayReason :type "EEndPlayReason Enum" :default "Destroyed"))
  ;[1 1 1] Starting and stopping the AR Session
  (`ARBlueprintLibrary.StopARSession`))

(event `TrackHands`
  (bind _lefthand (`self.LeftHand`))
  ;[1 1 1] Track our hands in 3D Space
  ;[1 1 1] Only track data if valid and from a hand
  (for _index (range 2)
    (bind _motioncontrollerdata (`HeadMountedDisplayFunctionLibrary.GetMotionControllerData` null (select `int` _index :`0` "Left" :`1` "Right" :!type "EControllerHand Enum")))
    (bind (_bvalid _devicename _applicationinstanceid _devicevisualtype _handindex _trackingstatus _gripposition _griprotation _aimposition _aimrotation _handkeypositions _handkeyrotations _handkeyradii) (break `XRMotionControllerData` _motioncontrollerdata))
    (if (and _bvalid (`|EnumEquality` _devicevisualtype "Hand"))
      ;[1 1 1] Retrieve the trackable points and their transform then posed the hand mesh to match the user's hand
      (bind _enumvalue (foreach `EHandKeypoint` false)
        (:`LoopBody`
          (bind _returnvalue (`self.RemoveSpaces` _enumvalue))
          ;;[1 1 1] Make sure the bone exists
          (if (`SceneComponent.DoesSocketExist` (`self.RightHand`) _returnvalue)
            (switch `EControllerHand` _handindex
              (:`Left`
                (bind _returnvalue_2 (`KismetMathLibrary.Conv_ByteToInt` _enumvalue))
                (bind _returnvalue_3 (`KismetMathLibrary.MakeTransform` (`|GetArrayItem` _handkeypositions _returnvalue_2) (`KismetMathLibrary.Quat_Rotator` (`|GetArrayItem` _handkeyrotations _returnvalue_2))))
                ;;[1 1 1] The left hand needs extra steps as the mesh was designed for the right hand
                (bind _adjustedtransform (`self.ConvertTransform` _returnvalue_3))
                (`PoseableMeshComponent.SetBoneTransformByName` _lefthand _returnvalue _adjustedtransform "ComponentSpace")
                ;;[1 1 1] Need to place the newly altered pose back to our world space.
                (`SceneComponent.K2_SetWorldLocation` _lefthand (0.0 0.0 0.0) false false))
              (:`Right`
                (`PoseableMeshComponent.SetBoneTransformByName` (`self.RightHand`) _returnvalue _returnvalue_3 "WorldSpace")))))))))

(event `EyeGazeTracking`
  ;[1 1 1] Eye Tracking
  (if (`EyeTrackerFunctionLibrary.IsEyeTrackerConnected`)
    (bind (_outgazedata _returnvalue) (`EyeTrackerFunctionLibrary.GetGazeData`))
    (`self.DetectBlink` _returnvalue)
    (if _returnvalue
      ;[1 1 1] Draw a line from our head in the direction our eyes are looking that is 5 meters long
      (bind _outhit (`KismetSystemLibrary.LineTraceSingle` (`self.HMDWorldLocation`) (+ (* (`.GazeDirection` (break `EyeTrackerGazeData` _outgazedata)) 500.0) (`SceneComponent.K2_GetComponentLocation` (`self.Camera`))) "TraceTypeQuery1"))
      (bind _output_get (set `self.EyeTrackingHit` _outhit))
      (bind (_bblockinghit _binitialoverlap _time _distance _location _impactpoint _normal _impactnormal _physmat _hitactor) (`GameplayStatics.BreakHitResult` _output_get))
      (if (`KismetSystemLibrary.DoesImplementInterface` _hitactor "/Game/WorldBuilder/Blueprint/Core/BPi_HoloLens.BPi_HoloLens_C")
        (message `/Game/WorldBuilder/Blueprint/Core/BPi_HoloLens.InteractWithUser` _hitactor "NewEnumerator0")))))

(event `HeadOrientationTracking`
  (bind _attachedactor (`self.AttachedActor`))
  ;[1 1 1] Head Tracking
  (bind _hmddata (`HeadMountedDisplayFunctionLibrary.GetHMDData` self))
  (if (break `XRHMDData` _hmddata)
    (bind _output_get (set `self.HMDWorldLocation` (`.Position` (break `XRHMDData` _hmddata))))
    (bind _outhit (`KismetSystemLibrary.LineTraceSingle` :`Start` _output_get :`End` (+ _output_get (* (`KismetMathLibrary.GetForwardVector` (`KismetMathLibrary.Quat_Rotator` (`.Rotation` (break `XRHMDData` _hmddata)))) 500.0)) :`TraceChannel` "TraceTypeQuery1" :`TraceColor` (struct :`G` 0.458208 :`B` 1.0 :`A` 1.0)))
    (set `self.HeadTrackingHit` _outhit)
    (`/Engine/EditorBlueprintResources/StandardMacros.IsValid` _attachedactor
      (:`Is Valid`
        (`self.K2_SetActorLocation` _attachedactor (`KismetMathLibrary.VInterpTo` (`self.K2_GetActorLocation` _attachedactor) (+ (`self.HMDWorldLocation`) (* (`SceneComponent.GetForwardVector` (`self.Camera`)) (`self.DistanceToTarget`))) (`GameplayStatics.GetWorldDeltaSeconds`) 3.0) false false)))))

(event `SpawnHandInteractions`
  (bind _returnvalue (`KismetMathLibrary.MakeTransform` (0.0 0.0 0.0)))
  ;[1 1 1] Spawn a hand interaction for both hands
  (bind _returnvalue_2 (`|SpawnActorFromClass` "/Script/UXTools.UxtHandInteractionActor" _returnvalue "Undefined" "OverrideRootScale" self true "Left" null))
  (bind _returnvalue_3 (`|SpawnActorFromClass` "/Script/UXTools.UxtHandInteractionActor" _returnvalue "Undefined" "OverrideRootScale" self true "Right" null))
  (bind _returnvalue_4 (`self.GetComponentByClass` _returnvalue_2 "/Script/UXTools.UxtFarCursorComponent"))
  ;[1 1 1] Cache the Far cursors from both hands
  (`/Engine/EditorBlueprintResources/StandardMacros.IsValid` _returnvalue_4
    (:`Is Valid`
      (set `self.LeftHandCursor` _returnvalue_4)
      (set `self.RightHandCursor` (`self.GetComponentByClass` _returnvalue_3 "/Script/UXTools.UxtFarCursorComponent")))))

(event `DetectBlink`
  (params (GazeTracking :type Boolean))
  ;[1 1 1] Blink detection
  (if GazeTracking
    ;[1 1 1] When eyes reopen, wait until user has finished blinking before reseting count
    (if (`self.EyesClosed`)
      (set `self.EyesClosed` false)
      (`KismetSystemLibrary.RetriggerableDelay` 0.5)
      (set `self.BlinkCount` 0))
    (else
      ;[1 1 1] Allow only .15 seconds for the eyes to be closed. If closed longer, Blueprint will ignore it.
      (if (not (`self.EyesClosed`))
        (set `self.EyesClosed` true)
        (`KismetSystemLibrary.Delay` 0.15)
        (if (not (`self.EyesClosed`))
          ;[1 1 1] Max of 3 blinks allowed
          (bind _result (`/Engine/EditorBlueprintResources/StandardMacros.IncrementInt` (`self.BlinkCount`))
            (:`  `
              (if (> _result 3)
                (set `self.BlinkCount` 0)
                (else
                  ;;[1 1 1] Pass on each blink for next step
                  (`self.UserBlinked`))))))))))

(event `ConfigureGestures`
  ;[1 1 1] Enable the Hold input
  (`HeadMountedDisplayFunctionLibrary.ConfigureGestures` (make `XRGestureConfig` false true)))

(event `InputAction|InteractWithLong`
  (params (Key :type "Key Structure"))
  (bind _returnvalue (`KismetStringLibrary.Contains` (`KismetTextLibrary.Conv_TextToString` (`KismetInputLibrary.Key_GetDisplayName` Key)) "Right"))
  ;[1 1 1] When the user presses and hold the tap gesture for a moment of time, call this input event to check if the overlapping actor is implementing BPi_HoloLens and if so, interact.
  (:`Pressed`
    (`self.CheckOverlapsFromHand` (`SceneComponent.K2_GetComponentLocation` (select `bool` _returnvalue :`false` (`self.LeftHandCursor`) :`true` (`self.RightHandCursor`) :!type "PrimitiveComponent Object Reference")) _returnvalue)))

(event `UserBlinked`
  ;[1 1 1] User has blink 1, 2, and/or three times. Now what?
  (switch `int` (`self.BlinkCount`)))

(event `CheckOverlapsFromHand`
  (params (HitLocation :type "Vector Structure") (RightHand :type Boolean))
  (bind _interactionoverlap (`self.InteractionOverlap`))
  ;[1 1 1] When the user presses and hold the tap gesture for a moment of time, call this input event to check if the overlapping actor is implementing BPi_HoloLens and if so, interact.
  (`SceneComponent.K2_SetWorldLocation` _interactionoverlap HitLocation false false)
  (for _array_element (`PrimitiveComponent.GetOverlappingActors` _interactionoverlap "/Script/Engine.Actor")
    (if (`KismetSystemLibrary.DoesImplementInterface` _array_element "/Game/WorldBuilder/Blueprint/Core/BPi_HoloLens.BPi_HoloLens_C")
      (message `/Game/WorldBuilder/Blueprint/Core/BPi_HoloLens.InteractWithObject` _array_element RightHand))))

(event `SpawnUI`
  ;[1 1 1] Spawning the UI to the world
  (bind _returnvalue (`|SpawnActorFromClass` "/Game/WorldBuilder/UI/Blueprints/BP_ObjectSpawner.BP_ObjectSpawner_C" (`KismetMathLibrary.MakeTransform` (0.0 0.0 0.0)) "Undefined" "OverrideRootScale" self null))
  ;[1 1 1] When the palm is facing up, render the tracked hands.
  (add `/Game/WorldBuilder/UI/Blueprints/BP_ObjectSpawner.ObjectSpawnerActive` _returnvalue (delegate `UIHandsActive`)))

(event `UIHandsActive`
  (params (Active :type Boolean))
  ;[1 1 1] When the palm is facing up, render the tracked hands.
  (set `self.RenderHands` Active))

(event `AddLocalAnchor`
  (params (`Anchor Name` :type String) (PlacementType :type Integer))
  ;[1 1 1] Called from BP_ToolBox: Add a new anchor to the scene. the Toolbox will provide a generated name and the type of placement to add to BP_Anchor
  ;;[1 1 1] 0 = Manual
  ;; 1 = Tap To Place
  ;;
  ;; See BP_Toolbox
  (if (and (`ARBlueprintLibrary.IsARPinLocalStoreSupported`) (`ARBlueprintLibrary.IsARPinLocalStoreReady`))
    (`self.SpawnAnchorForPlacement` `Anchor Name` PlacementType)
    (else
      (`KismetSystemLibrary.PrintString` "[BP_Pawn | AddLocalAnchor] + + + ARPin Local Store is NOT ready + + +") ; Warn User that the Local Store is not ready
    )))

(event `InputAction|InteractWithSingle`
  (params (Key :type "Key Structure"))
  (bind (_eyetrackinghit_bblockinghit _eyetrackinghit_binitialoverlap _eyetrackinghit_time _eyetrackinghit_distance _eyetrackinghit_location _eyetrackinghit_impactpoint _eyetrackinghit_normal _eyetrackinghit_impactnormal _eyetrackinghit_physmat _eyetrackinghit_hitactor) (`GameplayStatics.BreakHitResult` (`self.EyeTrackingHit`)))
  ;[1 1 1] Called from speech mapping "Single Interact"
  (:`Pressed`
    (message `/Game/WorldBuilder/Blueprint/Core/BPi_HoloLens.InteractWithObject` _eyetrackinghit_hitactor true)))

(event `SpawnAnchorForPlacement`
  (params (AnchorName :type String) (PlacementType :type Integer))
  (bind (_headtrackinghit_bblockinghit _headtrackinghit_binitialoverlap _headtrackinghit_time _headtrackinghit_distance _headtrackinghit_location _headtrackinghit_impactpoint _headtrackinghit_normal _headtrackinghit_impactnormal _headtrackinghit_physmat _headtrackinghit_hitactor _headtrackinghit_hitcomponent _headtrackinghit_hitbonename _headtrackinghit_hititem _headtrackinghit_faceindex _headtrackinghit_tracestart _headtrackinghit_traceend) (`GameplayStatics.BreakHitResult` (`self.HeadTrackingHit`)))
  ;[1 1 1] Spawn the anchor for placement by the end user. Does NOT create an anchor until it has been placed
  ;[1 1 1] Spawn the representation of the Anchor for the user to manupulate
  (bind _returnvalue (`|SpawnActorFromClass` "/Game/WorldBuilder/Blueprint/BP_Anchor.BP_Anchor_C" (`KismetMathLibrary.MakeTransform` (+ _headtrackinghit_tracestart (* (`KismetMathLibrary.GetForwardVector` (`KismetMathLibrary.FindLookAtRotation` _headtrackinghit_tracestart _headtrackinghit_traceend)) 60.0))) "AlwaysSpawn" "OverrideRootScale" null AnchorName null))
  (`/Game/WorldBuilder/Blueprint/BP_Anchor.AddInteractionComponent` _returnvalue PlacementType))

(event `InputAction|StatusCheck`
  (params (Key :type "Key Structure"))
  (bind (_eyetrackinghit_bblockinghit _eyetrackinghit_binitialoverlap _eyetrackinghit_time _eyetrackinghit_distance _eyetrackinghit_location _eyetrackinghit_impactpoint _eyetrackinghit_normal _eyetrackinghit_impactnormal _eyetrackinghit_physmat _eyetrackinghit_hitactor) (`GameplayStatics.BreakHitResult` (`self.EyeTrackingHit`)))
  ;[1 1 1] Call from speech mapping "Status Check"
  (:`Pressed`
    (if (`KismetSystemLibrary.DoesImplementInterface` _eyetrackinghit_hitactor "/Game/WorldBuilder/Blueprint/Core/BPi_HoloLens.BPi_HoloLens_C")
      ;;[1 1 1] If the actor that we are focus our EyeGaze on uses the interface, call GiveStatusUpdate on it alone. If not, broadcast to all
      (message `/Game/WorldBuilder/Blueprint/Core/BPi_HoloLens.GiveStatusUpdate` _eyetrackinghit_hitactor)
      (else
        (bind _outactors (`GameplayStatics.GetAllActorsWithInterface` "/Game/WorldBuilder/Blueprint/Core/BPi_HoloLens.BPi_HoloLens_C"))
        (for _array_element _outactors
          (message `/Game/WorldBuilder/Blueprint/Core/BPi_HoloLens.GiveStatusUpdate` _array_element))))))

(event `SaveLocalAnchor`
  (params (ComponentToPin :type "SceneComponent Object Reference") (DebugName :type Name))
  ;[1 1 1] After new Anchor has been placed, Save/Update transform
  (bind _returnvalue (`ARBlueprintLibrary.PinComponent` ComponentToPin (`SceneComponent.K2_GetComponentToWorld` ComponentToPin) null DebugName))
  (`KismetSystemLibrary.Delay` 0.5)
  (`ARBlueprintLibrary.SaveARPinToLocalStore` DebugName _returnvalue)
  ;[1 1 1] Add this new anchor to our array
  (`BlueprintMapLibrary.Map_Add` (`self.LoadedARPins`) DebugName _returnvalue))

(event `InputAction|HL_WorldBuilder`
  (params (Key :type "Key Structure"))
  (bind _bp_toolbox (`self.BP_Toolbox`))
  ;[1 1 1] Spawn BP_Toolbox when needed. When used, it will destroy. If not used, can be destroyed
  (:`Pressed`
    (`/Engine/EditorBlueprintResources/StandardMacros.IsValid` _bp_toolbox
      (:`Is Valid`
        (`self.K2_DestroyActor` _bp_toolbox))
      (:`Is Not Valid`
        (bind _returnvalue (`|SpawnActorFromClass` "/Game/WorldBuilder/UI/Blueprints/BP_Toolbox.BP_Toolbox_C" (`KismetMathLibrary.MakeTransform` (0.0 0.0 0.0)) "Undefined" "OverrideRootScale" null null))
        (bind _output_get (set `self.BP_Toolbox` _returnvalue))
        ;[1 1 1] When the user says or presses "Spawn", spawn the chosen class 1 meter in front of the head then destroy BP_Toolbox
        (add `/Game/WorldBuilder/UI/Blueprints/BP_Toolbox.UserPressedSpawn` _output_get (delegate `UserPressedSpawn_Event`))))))

(event `UserPressedSpawn_Event`
  (params (ToSpawn :type "Actor Class Reference"))
  (bind (_headtrackinghit_bblockinghit _headtrackinghit_binitialoverlap _headtrackinghit_time _headtrackinghit_distance _headtrackinghit_location _headtrackinghit_impactpoint _headtrackinghit_normal _headtrackinghit_impactnormal _headtrackinghit_physmat _headtrackinghit_hitactor _headtrackinghit_hitcomponent _headtrackinghit_hitbonename _headtrackinghit_hititem _headtrackinghit_faceindex _headtrackinghit_tracestart _headtrackinghit_traceend) (`GameplayStatics.BreakHitResult` (`self.HeadTrackingHit`)))
  ;[1 1 1] When the user says or presses "Spawn", spawn the chosen class 1 meter in front of the head then destroy BP_Toolbox
  (`|SpawnActorFromClass` ToSpawn (`KismetMathLibrary.MakeTransform` (+ _headtrackinghit_tracestart (* (`KismetMathLibrary.GetForwardVector` (`KismetMathLibrary.FindLookAtRotation` _headtrackinghit_tracestart _headtrackinghit_traceend)) 100.0))) "Undefined" "OverrideRootScale" null null))

(event `LoadLocalAnchors`
  (params (DisplayLoaded :type Boolean))
  ;[1 1 1] Load all Local Anchors and cache them into the Dictionary LoadedARPins for later use
  (`BlueprintMapLibrary.Map_Clear` (`self.LoadedARPins`))
  (bind _returnvalue (`ARBlueprintLibrary.LoadARPinsFromLocalStore`))
  (set `self.LoadedARPins` _returnvalue)
  ;[1 1 1] Update the anchor list
  (`self.CycleCurrentAnchorInToolbox`)
  ;[1 1 1] If the user wants to see the anchors after loading, spawn the anchor mesh
  (if DisplayLoaded
    (`self.SpawnAnchorMeshes`)))

(event `InputAction|UI_Cube`
  (params (Key :type "Key Structure"))
  (bind _bp_toolbox (`self.BP_Toolbox`))
  ;[1 1 1] Voice mappings to interact with BP_Toolbox
  (:`Pressed`
    (`/Engine/EditorBlueprintResources/StandardMacros.IsValid` _bp_toolbox
      (:`Is Valid`
        (`/Game/WorldBuilder/UI/Blueprints/BP_Toolbox.Voice_SetSwitch` _bp_toolbox 0) ; 0 is a cube
      ))))

(event `InputAction|UI_Sphere`
  (params (Key :type "Key Structure"))
  (bind _bp_toolbox (`self.BP_Toolbox`))
  ;[1 1 1] Voice mappings to interact with BP_Toolbox
  (:`Pressed`
    (`/Engine/EditorBlueprintResources/StandardMacros.IsValid` _bp_toolbox
      (:`Is Valid`
        (`/Game/WorldBuilder/UI/Blueprints/BP_Toolbox.Voice_SetSwitch` _bp_toolbox 1) ; 1 is a sphere
      ))))

(event `InputAction|UI_Spawn`
  (params (Key :type "Key Structure"))
  (bind _bp_toolbox (`self.BP_Toolbox`))
  ;[1 1 1] Voice mappings to interact with BP_Toolbox
  (:`Pressed`
    (`/Engine/EditorBlueprintResources/StandardMacros.IsValid` _bp_toolbox
      (:`Is Valid`
        (`/Game/WorldBuilder/UI/Blueprints/BP_Toolbox.SpawnButtonPressed` _bp_toolbox null null)))))

(event `SpawnAnchorMeshes`
  ;[1 1 1] If the user wants to see the pins after loading them, they have that option inside of BP_Toolkit
  (bind _values (`BlueprintMapLibrary.Map_Values` (`self.LoadedARPins`)))
  (for _array_element _values
    (bind _returnvalue (`ARPin.GetDebugName` _array_element))
    (bind _returnvalue_2 (`|SpawnActorFromClass` "/Game/WorldBuilder/Blueprint/BP_Anchor.BP_Anchor_C" (`KismetMathLibrary.MakeTransform` (0.0 0.0 0.0)) "AlwaysSpawn" "OverrideRootScale" null (`KismetStringLibrary.Conv_NameToString` _returnvalue) null))
    (`self.AttachActorToPin` (`/Game/WorldBuilder/Blueprint/BP_Anchor.Anchor` _returnvalue_2) _returnvalue)))

(event `self.ARTrackableNotify.OnUpdateTrackedGeometry`
  (params (TrackedGeometry :type "ARTrackedGeometry Object Reference"))
  (bind _returnvalue (`ARTrackedGeometry.GetUnderlyingMesh` TrackedGeometry))
  (bind (_returnvalue_additionalinfo _returnvalue_status) (break `ARSessionStatus` (`ARBlueprintLibrary.GetARSessionStatus`)))
  ;[1 1 1] Check if newly update mesh is valid
  (`/Engine/EditorBlueprintResources/StandardMacros.IsValid` _returnvalue
    (:`Is Valid`
      ;[1 1 1] Only proceed if the ARSession is running as expected
      (if (`|EnumEquality` _returnvalue_status "Running")
        ;[1 1 1] If the mesh is valid, add to arry
        (`KismetArrayLibrary.Array_AddUnique` (`self.Tracked Geometry`) _returnvalue)
        (if (`self.SpatialMappingRenderMesh`)
          (`self.SpatialMapping_SetVisibility` true))))))

(event `AttachActorToPin`
  (params (ComponentToPin :type "SceneComponent Object Reference") (DebugName :type Name))
  ;[1 1 1] Attach an actor to an anchor by searching through our Dictionary and finding the pin with a certain Name.
  (bind _values (`BlueprintMapLibrary.Map_Values` (`self.LoadedARPins`)))
  (for _array_element _values
    (if (== (`ARPin.GetDebugName` _array_element) DebugName)
      (bind _returnvalue (`ARPin.GetPinnedComponent` _array_element))
      (`/Engine/EditorBlueprintResources/StandardMacros.IsValid` _returnvalue
        (:`Is Valid`
          (`self.K2_AttachToComponent` (`ActorComponent.GetOwner` ComponentToPin) _returnvalue "None" "SnapToTarget" "SnapToTarget" "KeepRelative" true))
        (:`Is Not Valid`
          (`ARBlueprintLibrary.PinComponentToARPin` ComponentToPin _array_element))))))

(event `SpatialMapping_SetVisibility`
  (params (Visible :type Boolean))
  (bind _tracked_geometry (`self.Tracked Geometry`))
  ;[1 1 1] Allow the user to set a wireframe material to the mesh or remove it.
  (set `self.SpatialMappingRenderMesh` Visible)
  (for _array_element _tracked_geometry
    ;;[1 1 1] Check again to make sure that any scanned mesh is still valid. If not, remove from the array
    (`/Engine/EditorBlueprintResources/StandardMacros.IsValid` _array_element
      (:`Is Valid`
        (`PrimitiveComponent.SetMaterial` _array_element 0 (select `bool` (`self.SpatialMappingRenderMesh`) :`true` "/Game/WorldBuilder/Materials/Instance/M_EmissiveWire_Orange.M_EmissiveWire_Orange" :!type "MaterialInterface Object Reference")))
      (:`Is Not Valid`
        (`KismetArrayLibrary.Array_RemoveItem` _tracked_geometry _array_element)))))

(event `ToggleARSession`
  (params (Active :type Boolean))
  ;[1 1 1] Allow the user to start/pause the session
  (if Active
    (`ARBlueprintLibrary.StartARSession` "/Game/WorldBuilder/Assets/AR_SessionConfig.AR_SessionConfig")
    (else
      (`ARBlueprintLibrary.PauseARSession`))))

(event `DeleteLocalAnchor`
  (params (AnchorName :type Name) (RemovedBPAnchor :type "Actor Object Reference"))
  ;[1 1 1] Delete a single anchor using the menu on BP_Toolkit OR pressing the button on a BP_Anchor
  ;;[1 1 1] Remove the deleted anchor from the store
  (`ARBlueprintLibrary.RemoveARPinFromLocalStore` AnchorName)
  ;[1 1 1] If the InputObject is valid, the user pressed the button on the specific BP_Anchor. If it InNotValid, they are attempting to remove it through BP_Toolbox
  (`/Engine/EditorBlueprintResources/StandardMacros.IsValid` RemovedBPAnchor
    (:`Is Valid`
      (`self.K2_DestroyActor` RemovedBPAnchor))
    (:`Is Not Valid`
      (bind _outactors (`GameplayStatics.GetAllActorsOfClass` "/Game/WorldBuilder/Blueprint/BP_Anchor.BP_Anchor_C"))
      (for _array_element _outactors
        (if (`KismetStringLibrary.EqualEqual_StrStr` (`/Game/WorldBuilder/Blueprint/BP_Anchor.AnchorName` _array_element) (`KismetStringLibrary.Conv_NameToString` AnchorName))
          (`self.K2_DestroyActor` _array_element)))))
  ;[1 1 1] After the specific BP_Anchor is destroyed, update our cached Dictionary
  (`BlueprintMapLibrary.Map_Remove` (`self.LoadedARPins`) AnchorName)
  ;;[1 1 1] Update Toolbox's name display
  (`self.CycleCurrentAnchorInToolbox`))

(event `DeleteAllAnchors`
  ;[1 1 1] Delete all Local Anchors and destroy all the BP_Anchors
  (`ARBlueprintLibrary.RemoveAllARPinsFromLocalStore`)
  (bind _outactors (`GameplayStatics.GetAllActorsOfClass` "/Game/WorldBuilder/Blueprint/BP_Anchor.BP_Anchor_C"))
  (for _array_element _outactors
    (`self.K2_DestroyActor` _array_element))
  ;[1 1 1] Clear all the cached Pins
  (`BlueprintMapLibrary.Map_Clear` (`self.LoadedARPins`))
  ;[1 1 1] Update Toolbox's name display
  (`self.CycleCurrentAnchorInToolbox`))

(event `CycleCurrentAnchorInToolbox`
  (bind _bp_toolbox (`self.BP_Toolbox`))
  ;[1 1 1] Called in several locations, best to check if BP_Toolbox is valid before attempting the call
  (`/Engine/EditorBlueprintResources/StandardMacros.IsValid` _bp_toolbox
    (:`Is Valid`
      (`/Game/WorldBuilder/UI/Blueprints/BP_Toolbox.CycleAnchors` _bp_toolbox))))

(fn `ConvertTransform`
  (params (TrackedData :type "Transform Structure (by ref)"))
  (returns (AdjustedTransform :type "Transform Structure"))
  (bind (_returnvalue_location _returnvalue_rotation _returnvalue_scale) (`KismetMathLibrary.BreakTransform` (`KismetMathLibrary.ComposeTransforms` TrackedData (`SceneComponent.K2_GetComponentToWorld` (`self.LeftHand`)))))
  (return (`KismetMathLibrary.MakeTransform` _returnvalue_location _returnvalue_rotation (* _returnvalue_scale (1.0 -1.0 1.0)))))

(fn `UserConstructionScript`)