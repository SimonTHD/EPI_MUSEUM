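; BP_AnchorLocator pins itself to a named AR anchor once the player pawn has loaded that anchor.
; When an anchor is selected in AnchorToFind, BeginPlay starts a looping timer that polls BP_Pawn's LoadedARPins map every few seconds.
; On finding a key matching the enum's name, it passes its DefaultSceneRoot to the pawn's AttachActorToPin and pauses the timer.
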(event `self.ReceiveBeginPlay`
  ;[1 1 1] If we have not set an AnchorName to search for, do nothing. Otherwise, search for the anchor once every 3 seconds and repear
  (if (`|EnumInequality` (`self.AnchorToFind`) "NewEnumerator0")
    (bind _returnvalue (`KismetSystemLibrary.K2_SetTimerDelegate` (delegate `AnchorUpdated`) 3.0 true))
    (set `self.SearchTimer` _returnvalue)))

(event `AnchorUpdated`
  (bind _loadedarpins (`/Game/WorldBuilder/Blueprint/Pawns/BP_Pawn.LoadedARPins` (cast `/Game/WorldBuilder/Blueprint/Pawns/BP_Pawn` (`GameplayStatics.GetPlayerPawn` 0) :!pure true)))
  ;[1 1 1] Don't attempt the search until there are pins loaded into the map
  (if (> (`BlueprintMapLibrary.Map_Length` _loadedarpins) 0)
    (bind _keys (`BlueprintMapLibrary.Map_Keys` _loadedarpins))
    ;[1 1 1] When Anchors are loaded, check if there is one named what we need
    (if (`KismetArrayLibrary.Array_Contains` _keys (`KismetStringLibrary.Conv_StringToName` (`|GetEnumeratorNameAsString` (`self.AnchorToFind`))))
      ;[1 1 1] When found, call BP_Pawn and attach the parent of this ActorComponent to that pin and then pause the timer
      (`/Game/WorldBuilder/Blueprint/Pawns/BP_Pawn.AttachActorToPin` (cast `/Game/WorldBuilder/Blueprint/Pawns/BP_Pawn` (`GameplayStatics.GetPlayerPawn` 0) :!pure true) (`self.DefaultSceneRoot`) (`KismetStringLibrary.Conv_StringToName` (`|GetEnumeratorNameAsString` (`self.AnchorToFind`))))
      (`KismetSystemLibrary.K2_PauseTimerHandle` (`self.SearchTimer`)))))

(fn `UserConstructionScript`)